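; BP_JsonReadExample is an example actor that spawns test shapes from a JSON file at BeginPlay.
; It adds a child actor component, casts its actor to BP_JsonQuery, reads "input.json" and loops over the "objects" array.
; Each entry's type selects BP_TestCube or BP_TestSphere, spawned with a transform from GetTransform.
; Helper graphs hold nodes that assemble position, rotation and scale from three-element float arrays.
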(event `self.ReceiveBeginPlay`
  (bind _returnvalue (`AddComponent|NODE_AddChildActorComponent-0`))
  (bind _asbp_json_query (cast `/Game/Blueprints/BP_JsonQuery` (`ChildActorComponent.ChildActor` _returnvalue)))
  (set `/Game/Blueprints/BP_JsonQuery.ReadFile` "input.json" _asbp_json_query)
  (`/Game/Blueprints/BP_JsonQuery.ReadJson` _asbp_json_query)
  (for _array_element (`.ReturnValue` (`JsonFieldData.GetObjectArray` (`/Game/Blueprints/BP_JsonQuery.JsonData` _asbp_json_query) "objects"))
    (bind (_success _returnvalue_2) (`JsonFieldData.GetString` _array_element "type"))
    (if (== _returnvalue_2 "cube")
      (bind _transform (`self.GetTransform` _array_element))
      (`|SpawnActorFromClass` "/Game/Blueprints/BP_TestCube.BP_TestCube_C" _transform "Undefined" "OverrideRootScale" null null)
      (elif (== _returnvalue_2 "sphere")
        (`|SpawnActorFromClass` "/Game/Blueprints/BP_TestSphere.BP_TestSphere_C" _transform "Undefined" "OverrideRootScale" null null)))))

(fn `UserConstructionScript`)