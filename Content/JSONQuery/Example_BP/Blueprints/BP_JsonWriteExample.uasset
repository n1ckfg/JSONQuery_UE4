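; Example actor that saves the level's BP_TestCube and BP_TestSphere actors to JSON on BeginPlay.
; After a short delay it spawns a BP_JsonQuery child actor and gathers both actor classes.
; The ActorToJson macro turns each into an object with type, position, rotation and scale float arrays.
; These objects form an "objects" array, minus a placeholder first element, which BP_JsonQuery writes through WriteJson.
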(event `self.ReceiveBeginPlay`
  (`KismetSystemLibrary.Delay` 1.0)
  (bind _returnvalue (`AddComponent|NODE_AddChildActorComponent-0`))
  (bind _asbp_json_query (cast `/Game/JSONQuery/Blueprints/BP_JsonQuery` (`ChildActorComponent.ChildActor` _returnvalue)))
  (bind _output_get (set `self.ObjectArray` (`|MakeArray` (`JsonFieldData.Create`))))
  (bind _outactors (`GameplayStatics.GetAllActorsOfClass` "/Game/JSONQuery/Example_BP/Blueprints/BP_TestCube.BP_TestCube_C"))
  (for _array_element _outactors
    (bind _jsondata (`self.ActorToJson` "cube" (`self.GetTransform` _array_element))
      (:`ExecOut`
        (`KismetArrayLibrary.Array_Add` _output_get _jsondata))))
  (bind _outactors_2 (`GameplayStatics.GetAllActorsOfClass` "/Game/JSONQuery/Example_BP/Blueprints/BP_TestSphere.BP_TestSphere_C"))
  (for _array_element_2 _outactors_2
    (bind _jsondata_2 (`self.ActorToJson` "sphere" (`self.GetTransform` _array_element_2))
      (:`ExecOut`
        (`KismetArrayLibrary.Array_Add` _output_get _jsondata_2))))
  (`KismetArrayLibrary.Array_Remove` _output_get)
  (bind _returnvalue_2 (`JsonFieldData.SetObjectArray` (`JsonFieldData.Create`) "objects" _output_get))
  (set `/Game/JSONQuery/Blueprints/BP_JsonQuery.JsonData` _returnvalue_2 _asbp_json_query)
  (`/Game/JSONQuery/Blueprints/BP_JsonQuery.WriteJson` _asbp_json_query))

(fn `UserConstructionScript`)